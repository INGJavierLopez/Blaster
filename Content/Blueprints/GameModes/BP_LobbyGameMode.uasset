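; BP_LobbyGameMode is the lobby game mode, and its graph holds only debug readouts of player group assignments.
; On Tick, when player 0's pawn is locally controlled with authority, it prints each PlayerGroupMap entry from BP_BlasterGameInstance as Group A, Group B or none.
; Disconnected leftovers cover a return-to-main-menu widget and prints for session state, connection count and map totals.
; BeginPlay and the Prueba event are empty.
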(event `self.ReceiveBeginPlay`)

(event `self.Prueba`
  (params (dato :type Integer) (DeltaSeconds :type "Float (single-precision)")))

(event `self.ReceiveTick`
  (params (DeltaSeconds :type "Float (single-precision)"))
  (bind _returnvalue (`Controller.K2_GetPawn` (`GameplayStatics.GetPlayerController` 0)))
  (`/Engine/EditorBlueprintResources/StandardMacros.IsValid` _returnvalue
    (:`Is Valid`
      (if (and (`Pawn.IsLocallyControlled` _returnvalue) (`self.HasAuthority` _returnvalue))
        (bind _asbp_blaster_game_instance (cast `/Game/Blueprints/GameInstance/BP_BlasterGameInstance` (`GameplayStatics.GetGameInstance`)))
        (bind _playergroupmap (`BlasterGameInstance.PlayerGroupMap` _asbp_blaster_game_instance))
        (bind _keys (`BlueprintMapLibrary.Map_Keys` _playergroupmap))
        (bind _values (`BlueprintMapLibrary.Map_Values` _playergroupmap))
        (for (_array_element _array_index) _keys
          (`KismetSystemLibrary.PrintString` (`KismetStringLibrary.Concat_StrStr` "Key: " _array_element " | Valor: " (select `EGroup` (`|GetArrayItem` _values _array_index) :`EG_A` "Grupo A" :`EG_B` "Grupo B" :`EG_NG` "NG") " \n") true true (struct :`G` 0.66 :`B` 1.0 :`A` 1.0) DeltaSeconds))))))

(fn `UserConstructionScript`)