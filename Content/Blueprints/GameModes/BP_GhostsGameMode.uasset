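; BP_GhostsGameMode is a game mode Blueprint for the Blaster project that currently adds only on-screen debug output.
; Tick calls the parent tick, then prints the inherited-looking CountdownTime value every frame, using delta time as the display duration.
; A disconnected branch would print each player's team and the player count from BP_BlasterGameState, but it never runs.
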(event `self.ReceiveTick`
  (params (DeltaSeconds :type "Float (single-precision)"))
  (`parent.ReceiveTick` DeltaSeconds)
  (`KismetSystemLibrary.PrintString` (`KismetStringLibrary.Concat_StrStr` "Countdown Time: " (`KismetStringLibrary.Conv_DoubleToString` (`self.CountdownTime`))) true true (struct :`G` 0.66 :`B` 1.0 :`A` 1.0) DeltaSeconds))

(fn `UserConstructionScript`)