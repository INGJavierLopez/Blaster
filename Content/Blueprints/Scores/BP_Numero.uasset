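; BP_Numero is a physics-driven score number that acts out an end-of-round show as winner or loser.
; Attack launches the winner along Y by team; on hitting another BP_Numero, the winner freezes, the loser gets knocked by an impulse, and both request a reset.
; RequestReset waits, eases the mesh back to its stored location, then restores physics and hit reaction.
; Expand uses timelines to scale the winner up and back down.
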(event `self.ReceiveBeginPlay`
  (set `self.DefaultLocation` (`SceneComponent.K2_GetComponentLocation` (`self.StaticMesh`)))
  (`KismetSystemLibrary.Delay` 1.0)
  (if (`|EnumEquality` (`self.NumberType`) "NewEnumerator0")
    _))

(event `Attack`
  (params (Selection :type "/Game/Blueprints/Scores/E_NumberTyoe Enum" :default "NewEnumerator0"))
  (bind _returnvalue (* (`self.ImpulseForce`) 100000.0))
  ;[1 1 1] Attack
  (bind _output_get (set `self.NumberType` Selection))
  (set `self.EndRoundShowType` "NewEnumerator0")
  (switch `/Game/Blueprints/Scores/E_NumberTyoe` _output_get
    (:`NewEnumerator0`
      (`PrimitiveComponent.AddImpulse` (`self.StaticMesh`) (`KismetMathLibrary.MakeVector` 0.0 (select `/Game/Blueprints/Scores/E_Team` (`self.Team`) :`NewEnumerator0` (* _returnvalue -1.0) :`NewEnumerator1` _returnvalue)) "None" false))))

(event `self.StaticMesh.OnComponentHit`
  (params (HitComponent :type "PrimitiveComponent Object Reference") (OtherActor :type "Actor Object Reference") (OtherComp :type "PrimitiveComponent Object Reference") (NormalImpulse :type "Vector Structure") (Hit :type "HitResult Structure (by ref)"))
  ;[1 1 1] Hit Event
  ;[1 1 1] Handle Hit Between Numbers
  (bind _asbp_numero (cast `/Game/Blueprints/Scores/BP_Numero` OtherActor))
  (switch `/Game/Blueprints/Scores/EEndRoundShowType` (`self.EndRoundShowType`)
    (:`NewEnumerator0`
      (if (`self.bCanReactToHit`)
        ;[1 1 1] Disable Hits
        (set `self.bCanReactToHit` false)
        (switch `/Game/Blueprints/Scores/EEndRoundShowType` (`self.EndRoundShowType`)
          (:`NewEnumerator0`
            ;[1 1 1] Request Reset for both
            (`self.RequestReset` _asbp_numero)
            (`self.RequestReset`)
            (switch `/Game/Blueprints/Scores/E_NumberTyoe` (`self.NumberType`)
              (:`NewEnumerator0`
                (`PrimitiveComponent.SetSimulatePhysics` (`self.StaticMesh`) false))
              (:`NewEnumerator1`
                (`PrimitiveComponent.AddImpulse` (`self.StaticMesh`) (`KismetMathLibrary.MakeVector` 0.0 (select `/Game/Blueprints/Scores/E_Team` (`self.Team`) :`NewEnumerator0` 100000.0 :`NewEnumerator1` -100000.0)) "None" false)))))))))

(event `RequestReset`
  ;[1 1 1] Request Rest
  (`KismetSystemLibrary.Delay` 5.0)
  (`PrimitiveComponent.SetSimulatePhysics` (`self.StaticMesh`) false)
  (`KismetSystemLibrary.MoveComponentTo` (`self.StaticMesh`) (`self.DefaultLocation`) (struct) true true)
  (`KismetSystemLibrary.Delay` 1.0)
  ;[1 1 1] Reset Physics and Hit Reaction
  (`PrimitiveComponent.SetSimulatePhysics` (`self.StaticMesh`) true)
  (set `self.bCanReactToHit` true))

(event `Expand`
  (params (Selection :type "/Game/Blueprints/Scores/E_NumberTyoe Enum" :default "NewEnumerator0"))
  ;[1 1 1] Expand
  (switch `/Game/Blueprints/Scores/E_NumberTyoe` Selection
    (:`NewEnumerator0`
      (bind (_direction _alpha) (`Timeline|ExpandBody` :!via `PlayFromStart`)
        (:`Update`
          (`SceneComponent.SetWorldScale3D` (`self.StaticMesh`) (`KismetMathLibrary.VLerp` (1.0 1.0 1.0) (10.0 10.0 10.0) _alpha)))
        (:`Finished`
          (`self.RequestResetGravity`))))))

(event `RequestResetGravity`
  (bind (_direction _alpha) (`Timeline|ResetScaleTL`)
    (:`Update`
      (`SceneComponent.SetWorldScale3D` (`self.StaticMesh`) (`KismetMathLibrary.VLerp` (10.0 10.0 10.0) (1.0 1.0 1.0) _alpha)))))

(fn `CheckNumberCanBeHItted`
  (returns (NewParam :type Boolean))
  (if (`self.bCanReactToHit`)
    (set `self.bCanReactToHit` false)))

(fn `UserConstructionScript`
  (`StaticMeshComponent.SetStaticMesh` (`self.StaticMesh`) (`self.Mesh`)))