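; BP_ScoreCamera is a score set piece with red and blue BP_Numero child actors and a base, walls and roof.
; The construction script caches both number actors and assigns their teams.
; Two seconds after BeginPlay, it calls Expand on both numbers, then enables physics on the set meshes.
; SetMeshesPhysics enables simulation whatever its Activate input; the Attack calls are unwired.
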(event `self.ReceiveBeginPlay`
  (`KismetSystemLibrary.Delay` 2.0)
  (`/Game/Blueprints/Scores/BP_Numero.Expand` (`self.BlueTeamNumRef`) "NewEnumerator0")
  (`/Game/Blueprints/Scores/BP_Numero.Expand` (`self.RedTeamNumRef`) "NewEnumerator1")
  (`self.SetMeshesPhysics` true))

(fn `SetMeshesPhysics`
  (params (Activate :type Boolean))
  (bind _paredroja (`self.ParedRoja`))
  (if Activate
    (`PrimitiveComponent.SetSimulatePhysics` _paredroja true)
    (`PrimitiveComponent.SetSimulatePhysics` (`self.ParedTrasera`) true)
    (`PrimitiveComponent.SetSimulatePhysics` (`self.Techo`) true)
    (`PrimitiveComponent.SetSimulatePhysics` (`self.Base`) true)
    (else
      (`PrimitiveComponent.SetSimulatePhysics` _paredroja true)
      (`PrimitiveComponent.SetSimulatePhysics` (`self.ParedTrasera`) true)
      (`PrimitiveComponent.SetSimulatePhysics` (`self.Techo`) true)
      (`PrimitiveComponent.SetSimulatePhysics` (`self.Base`) true))))

(fn `UserConstructionScript`
  (set `self.BlueTeamNumRef` (cast `/Game/Blueprints/Scores/BP_Numero` (`ChildActorComponent.ChildActor` (`self.BlueTeamNum`)) :!pure true))
  (bind _asbp_numero (cast `/Game/Blueprints/Scores/BP_Numero` (`ChildActorComponent.ChildActor` (`self.RedTeamNum`))))
  (set `self.RedTeamNumRef` _asbp_numero)
  (set `/Game/Blueprints/Scores/BP_Numero.Team` "NewEnumerator1" (`self.BlueTeamNumRef`))
  (set `/Game/Blueprints/Scores/BP_Numero.Team` "NewEnumerator0" (`self.RedTeamNumRef`)))