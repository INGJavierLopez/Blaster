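; BP_BlasterGameState is the game state for the Blaster game, here used as an on-screen debug readout of the players.
; Every tick it prints the player count, then loops PlayerArray, casting each player state and its pawn to the Blaster classes.
; For each character it prints Ghost status and team name, colored by Ghost and marking the locally controlled one, with messages lasting one frame.
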(event `self.ReceiveTick`
  (params (DeltaSeconds :type "Float (single-precision)"))
  (bind _playerarray (`self.PlayerArray`))
  (`KismetSystemLibrary.PrintString` (`KismetStringLibrary.Concat_StrStr` "PLAYERS: " (`KismetStringLibrary.Conv_IntToString` (`KismetArrayLibrary.Array_Length` _playerarray))) true false (struct :`R` 1.0 :`B` 0.595333 :`A` 1.0) DeltaSeconds)
  (for _array_element _playerarray
    (bind _asbp_blaster_player_state (cast `/Game/Blueprints/PlayerState/BP_BlasterPlayerState` _array_element))
    (bind _asbp_blaster_character (cast `/Game/Blueprints/Character/BP_BlasterCharacter` (`PlayerState.GetPawn` _asbp_blaster_player_state)))
    (if (`Pawn.IsLocallyControlled` _asbp_blaster_character)
      (if (`BlasterCharacter.bGhost` _asbp_blaster_character)
        (bind _team (`BlasterPlayerState.Team` _asbp_blaster_player_state))
        (`KismetSystemLibrary.PrintString` (`KismetStringLibrary.Concat_StrStr` "SOY YO GHOST  |||  " (`KismetStringLibrary.Conv_NameToString` (`|GetEnumeratorName` _team))) true true (struct :`R` 1.0 :`A` 1.0) DeltaSeconds)
        (else
          (`KismetSystemLibrary.PrintString` (`KismetStringLibrary.Concat_StrStr` "SOY YO NO GHOST |||  " (`KismetStringLibrary.Conv_NameToString` (`|GetEnumeratorName` _team))) true true (struct :`B` 1.0 :`A` 1.0) DeltaSeconds)))
      (elif (`BlasterCharacter.bGhost` _asbp_blaster_character)
        (`KismetSystemLibrary.PrintString` (`KismetStringLibrary.Concat_StrStr` "GHOST  |||  " (`KismetStringLibrary.Conv_NameToString` (`|GetEnumeratorName` _team))) true true (struct :`R` 1.0 :`A` 1.0) DeltaSeconds)
        (else
          (`KismetSystemLibrary.PrintString` (`KismetStringLibrary.Concat_StrStr` "NO GHOST |||  " (`KismetStringLibrary.Conv_NameToString` (`|GetEnumeratorName` _team))) true true (struct :`B` 0.974 :`A` 1.0) DeltaSeconds)))))
  (`KismetSystemLibrary.PrintString` "||||||||||||||||" true true (struct :`R` 0.979645 :`G` 1.0 :`B` 0.878076 :`A` 1.0) DeltaSeconds))

(fn `UserConstructionScript`)